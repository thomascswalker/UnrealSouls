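; Souls-like player character with camera-relative movement, sprinting, stamina-costed rolling and jumping, which also creates the main HUD on BeginPlay.
; Sprint and roll use hold and tap inputs; releasing sprint opens a brief threshold during which the roll input jumps instead.
; StartRoll changes speed and acceleration, plays a montage and pauses stamina replenishment, while Tick pushes the character forward.
; StopRoll restores these settings but has no caller in this file.
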(event Input|EnhancedActionEvents|EnhancedInputActionIA_Move
  (params (ActionValue :type Vector%202D%20Structure) (ElapsedSeconds :type Float%20%28double-precision%29) (TriggeredSeconds :type Float%20%28double-precision%29) (InputAction :type Input%20Action%20Object%20Reference :default "/Game/Input/Actions/IA_Move.IA_Move"))
  (bind (_x _y) (Math|Vector2D|BreakVector2D ActionValue))
  (bind _returnvalue (Pawn|GetController))
  ;[1 1 1] Movement
  (:Triggered
    (Pawn|Input|AddMovementInput (Transformation|GetActorForwardVector _returnvalue) _y false)
    (Pawn|Input|AddMovementInput (Transformation|GetActorRightVector _returnvalue) _x false)))

(event Input|EnhancedActionEvents|EnhancedInputActionIA_Look
  (params (ActionValue :type Vector%202D%20Structure) (ElapsedSeconds :type Float%20%28double-precision%29) (TriggeredSeconds :type Float%20%28double-precision%29) (InputAction :type Input%20Action%20Object%20Reference :default "/Game/Input/Actions/IA_Look.IA_Look"))
  (bind (_x _y) (Math|Vector2D|BreakVector2D ActionValue))
  ;[1 1 1] Looking
  (:Triggered
    (Pawn|Input|AddControllerYawInput _x)
    (Pawn|Input|AddControllerPitchInput _y)))

(event Input|EnhancedActionEvents|EnhancedInputActionIA_Sprint
  (params (ActionValue :type Boolean) (ElapsedSeconds :type Float%20%28double-precision%29) (TriggeredSeconds :type Float%20%28double-precision%29) (InputAction :type Input%20Action%20Object%20Reference :default "/Game/Input/Actions/IA_Sprint.IA_Sprint"))
  ;[1 1 1] Sprinting
  (:Triggered
    (Variables|Movement|SetbIsSprinting true)
    (Variables|/Script/Engine.CharacterMovementComponent|SetMaxWalkSpeed (Variables|Character|GetCharacterMovement) (Variables|Movement|GetSprintSpeed)) ; Sprint
  )
  (:Completed
    (Variables|Movement|SetbCanJump true)
    (Utilities|FlowControl|Delay (Variables|Movement|GetJumpThreshold)) ; Delay to allow jumping during the jump threshold
    (Variables|Movement|SetbIsSprinting false)
    (Variables|/Script/Engine.CharacterMovementComponent|SetMaxWalkSpeed (Variables|Character|GetCharacterMovement) (Variables|Movement|GetRunSpeed)) ; Run
    (Variables|Movement|SetbCanJump false)))

(event Input|EnhancedActionEvents|EnhancedInputActionIA_Roll
  (params (ActionValue :type Boolean) (ElapsedSeconds :type Float%20%28double-precision%29) (TriggeredSeconds :type Float%20%28double-precision%29) (InputAction :type Input%20Action%20Object%20Reference :default "/Game/Input/Actions/IA_Roll.IA_Roll"))
  ;[1 1 1] Rolling & Jumping
  (:Completed
    (bind _returnvalue (Movement|CanRoll))
    (if _returnvalue
      (Movement|StartRoll true)
      (else
        (bind _canjump (Movement|CanPlayerJump))
        (if _canjump
          (Character|Jump))))))

(event EventBeginPlay
  (Variables|/Script/Engine.CharacterMovementComponent|SetMaxWalkSpeed (Variables|Character|GetCharacterMovement) (Variables|Movement|GetRunSpeed))
  (bind _returnvalue (UserInterface|CreateWidget "/Game/Blueprints/HUD/WBP_MainHUD.WBP_MainHUD_C" 0 self))
  (UserInterface|Viewport|AddtoViewport _returnvalue 0))

(event EventTick
  (params (DeltaSeconds :type Float%20%28single-precision%29))
  (if (Variables|Movement|GetbIsRolling)
    (Movement|Roll)))

(fn ConstructionScript)

(fn CanRoll
  (return (Math|Boolean|ANDBoolean (Movement|IsMoving) (not (Variables|Movement|GetbIsRolling)) (not (Variables|Movement|GetbIsJumping)) (not (Variables|Movement|GetbCanJump)) (> (Variables|/Script/UnrealSouls.StatusComponent|GetValue (Variables|Default|GetBP_StaminaComponent)) 0.0))))

(fn CanPlayerJump
  (return (Math|Boolean|ANDBoolean (Movement|IsMoving) (not (Variables|Movement|GetbIsRolling)) (not (Variables|Movement|GetbIsJumping)) (Variables|Movement|GetbCanJump))))

(fn StartRoll
  (params (DepleteStamina :type Boolean))
  (bind _charactermovement (Variables|Character|GetCharacterMovement))
  (Variables|Movement|SetbIsSprinting false)
  (Variables|Movement|SetbIsRolling true)
  (Variables|/Script/Engine.CharacterMovementComponent|SetMaxWalkSpeed _charactermovement (Variables|Movement|GetRollSpeed))
  (Variables|/Script/Engine.CharacterMovementComponent|SetMaxAcceleration _charactermovement (Variables|Movement|GetRollAcceleration))
  (Animation|PlayMontage "/Game/Blueprints/AM_Roll.AM_Roll" "None" 1.0)
  (if DepleteStamina
    (Class|StatusComponent|Deplete (Variables|Default|GetBP_StaminaComponent) (Variables|Attributes|GetRollCost))
    (Variables|/Script/UnrealSouls.StatusComponent|SetbCanReplenish (Variables|Default|GetBP_StaminaComponent) false)))

(fn StopRoll
  (bind _charactermovement (Variables|Character|GetCharacterMovement))
  (Variables|Movement|SetbIsRolling false)
  (Variables|/Script/Engine.CharacterMovementComponent|SetMaxWalkSpeed _charactermovement (Variables|Movement|GetRunSpeed))
  (Variables|/Script/Engine.CharacterMovementComponent|SetMaxAcceleration _charactermovement (Variables|Movement|GetDefaultAcceleration))
  (Variables|Animation|SetCurrentMontage 0)
  (Variables|/Script/UnrealSouls.StatusComponent|SetbCanReplenish (Variables|Default|GetBP_StaminaComponent) true))

(fn Roll
  (Pawn|Input|AddMovementInput (Transformation|GetActorForwardVector) (Variables|Movement|GetRollSpeed) false))

(fn IsMoving
  (return (> (Math|Vector|VectorLength (Transformation|GetVelocity)) 1.0)))

(fn PlayMontage
  (params (Montage :type Anim%20Montage%20Object%20Reference) (StartSectionName :type Name) (PlayRate :type Float%20%28double-precision%29))
  (if (not (Animation|Montage|MontageIsPlaying (Components|SkeletalMesh|GetAnimInstance (Variables|Character|GetMesh)) Montage))
    (bind _output_get (Variables|Animation|SetCurrentMontage Montage))
    (bind _returnvalue (Animation|PlayAnimMontage _output_get PlayRate StartSectionName))
    (return _returnvalue)))