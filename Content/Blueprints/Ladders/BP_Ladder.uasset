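; Climbable ladder actor for UnrealSoulsCharacter, offering a "Climb" action.
; The construction script builds rungs from count and height, sizes the collider, and adds top and bottom exit boxes plus arrows marking start and exit points.
; BindCharacter and UnbindCharacter return locations, rotation and start or end montage by the character's end of the ladder.
; Interact and exit-overlap events only cast the actor; the OnStartClimb and OnEndClimb calls are unconnected.
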(event Custom|OnOverlapExitCollider
  (params (OverlappedComponent :type Primitive%20Component%20Object%20Reference) (OtherActor :type Actor%20Object%20Reference) (OtherComp :type Primitive%20Component%20Object%20Reference) (OtherBodyIndex :type Integer) (bFromSweep :type Boolean) (SweepResult :type Hit%20Result%20Structure%20%28by%20ref%29))
  ;[0 0 0] Exit climb
  (Utilities|Casting|CastToUnrealSoulsCharacter OtherActor)
  (if true
    _))

(event EventBeginPlay
  (Collision|BindEventtoOnComponentBeginOverlap (Variables|Default|GetBottomExitCollider) (EventDispatchers|CreateEvent :!event Custom|OnOverlapExitCollider))
  (Collision|BindEventtoOnComponentBeginOverlap (Variables|Default|GetTopExitCollider) (EventDispatchers|CreateEvent :!event Custom|OnOverlapExitCollider)))

(event EventInteract
  (params (OtherActor :type Actor%20Object%20Reference))
  ;[0 0 0] Enter climb
  (Utilities|Casting|CastToUnrealSoulsCharacter OtherActor)
  (if true
    _))

(fn ConstructionScript
  (bind _rungcount (Variables|Ladder|GetRungCount))
  (bind _rungheight (Variables|Ladder|GetRungHeight))
  (bind _rungheight_2 (Variables|Ladder|GetRungHeight))
  (bind _returnvalue (* _rungheight_2 _rungcount))
  (bind _returnvalue_2 (/ _returnvalue 2.0))
  (Utilities|FlowControl|Sequence
    (:then_0
      (for _index (range 0 (Variables|Ladder|GetRungCount))
        (bind _returnvalue_3 (AddComponent|AddStaticMeshComponent false (Math|Transform|MakeTransform (+ (Math|Vector|MakeVector 0.0 0.0 (* _index (Variables|Ladder|GetRungHeight))) (Variables|Default|GetMeshOffset)) "0.000000,90.000000,0.000000" "1.000000,1.000000,1.000000")))
        (Components|StaticMesh|SetStaticMesh _returnvalue_3 (Variables|Ladder|GetRungMesh))
        (Rendering|Material|SetMaterial _returnvalue_3 0 (Variables|Ladder|GetMaterial))))
    (:then_1
      (Transformation|SetRelativeLocation (Variables|Default|GetCollider) (Math|Vector|MakeVector 0.0 0.0 _returnvalue_2) false false)
      (Components|Capsule|SetCapsuleHalfHeight (Variables|Default|GetCollider) (+ _returnvalue_2 1e+02) true))
    (:then_2
      ;[1 1 1] Bottom exit collider
      (bind _returnvalue_4 (AddComponent|AddBoxComponent false (Math|Transform|MakeTransform (Math|Vector|MakeVector -5e+01 0.0 0.0) "0, 0, 0" "1.000000,1.000000,1.000000")))
      (bind _output_get (Variables|Default|SetBottomExitCollider _returnvalue_4))
      (Components|Box|SetBoxExtent _output_get "50.000000,50.000000,25.000000" true)
      ;[1 1 1] Top exit collider
      (bind _returnvalue_5 (AddComponent|AddBoxComponent false (Math|Transform|MakeTransform (Math|Vector|MakeVector -5e+01 0.0 (+ (* (Variables|Ladder|GetRungCount) _rungheight) (* _rungheight 3.0))) "0, 0, 0" "1.000000,1.000000,1.000000")))
      (bind _output_get_2 (Variables|Default|SetTopExitCollider _returnvalue_5))
      (Components|Box|SetBoxExtent _output_get_2 "50.000000,50.000000,25.000000" true)
      (Variables|Ladder|SetTopExitLocation (Math|Vector|MakeVector 5e+01 0.0 (+ (* (Variables|Ladder|GetRungCount) (Variables|Ladder|GetRungHeight)) 5e+01)))
      (Variables|Ladder|SetBottomExitLocation (Math|Vector|MakeVector -1e+02 0.0 1e+02))
      (Variables|Ladder|SetTopStartLocation (Math|Vector|MakeVector -66.0 0.0 (- (* (Variables|Ladder|GetRungCount) (Variables|Ladder|GetRungHeight)) 1.2e+02)))
      (Variables|Ladder|SetBottomStartLocation (Math|Vector|MakeVector -75.0 0.0 1.5e+02))
      (Utilities|FlowControl|Sequence
        (:then_0
          (bind _returnvalue_6 (AddComponent|AddArrowComponent false (Math|Transform|MakeTransform (Variables|Ladder|GetTopExitLocation) "0, 0, 0" "1.000000,1.000000,1.000000")))
          (bind _output_get_3 (Variables|Default|SetTopExitComponent _returnvalue_6))
          (Components|Arrow|SetArrowColor(LinearColor) _output_get_3 "(R=1.000000,G=0.036947,B=0.000000,A=1.000000)")
          (Development|SetHiddeninGame _output_get_3 false false))
        (:then_1
          (bind _returnvalue_7 (AddComponent|AddArrowComponent false (Math|Transform|MakeTransform (Variables|Ladder|GetBottomExitLocation) "0, 0, 0" "1.000000,1.000000,1.000000")))
          (bind _output_get_4 (Variables|Default|SetBottomExitComponent _returnvalue_7))
          (Components|Arrow|SetArrowColor(LinearColor) _output_get_4 "(R=0.155967,G=1.000000,B=0.000000,A=1.000000)")
          (Development|SetHiddeninGame _output_get_4 false false))
        (:then_2
          (bind _returnvalue_8 (AddComponent|AddArrowComponent false (Math|Transform|MakeTransform (Variables|Ladder|GetTopStartLocation) "0, 0, 0" "1.000000,1.000000,1.000000")))
          (bind _output_get_5 (Variables|Default|SetTopStartComponent _returnvalue_8))
          (Components|Arrow|SetArrowColor(LinearColor) _output_get_5 "(R=1.000000,G=0.000000,B=0.842125,A=1.000000)")
          (Development|SetHiddeninGame _output_get_5 false false))
        (:then_3
          (bind _returnvalue_9 (AddComponent|AddArrowComponent false (Math|Transform|MakeTransform (Variables|Ladder|GetBottomStartLocation) "0, 0, 0" "1.000000,1.000000,1.000000")))
          (bind _output_get_6 (Variables|Default|SetBottomStartComponent _returnvalue_9))
          (Components|Arrow|SetArrowColor(LinearColor) _output_get_6 "(R=0.000000,G=0.119408,B=1.000000,A=1.000000)")
          (Development|SetHiddeninGame _output_get_6 false false))))))

(fn GetActionText
  (return "Climb"))

(fn BindCharacter
  (params (Character :type Unreal%20Souls%20Character%20Object%20Reference))
  (LocalVariables|SetRotation (Transformation|GetActorRotation))
  (bind _position (CallFunction|GetCharacterPosition Character))
  (switch Utilities|FlowControl|Switch|Switchon _position
    (:Bottom
      (return (Variables|Ladder|GetBottomExitLocation) (Variables|Ladder|GetBottomStartLocation) (LocalVariables|GetRotation) "/Game/Blueprints/Player/Animations/AM_ClimbUpStart.AM_ClimbUpStart"))
    (:Top
      (return (Variables|Ladder|GetTopExitLocation) (Variables|Ladder|GetTopStartLocation) (LocalVariables|GetRotation) "/Game/Blueprints/Player/Animations/AM_ClimbDownStart.AM_ClimbDownStart"))))

(fn GetCharacterPosition
  (params (Character :type Unreal%20Souls%20Character%20Object%20Reference))
  (if (Collision|IsOverlappingActor (Variables|Default|GetTopExitCollider) Character :!class /Script/Engine.PrimitiveComponent)
    (return 0)
    (elif (Collision|IsOverlappingActor (Variables|Default|GetBottomExitCollider) Character :!class /Script/Engine.PrimitiveComponent)
      (return 0)
      (else
        (return 0)))))

(fn UnbindCharacter
  (params (Character :type Unreal%20Souls%20Character%20Object%20Reference))
  (LocalVariables|SetRotation (Transformation|GetActorRotation))
  (bind _position (CallFunction|GetCharacterPosition Character))
  (switch Utilities|FlowControl|Switch|Switchon _position
    (:Bottom
      (return (Variables|Ladder|GetBottomExitLocation) (Variables|Ladder|GetBottomStartLocation) (LocalVariables|GetRotation) "/Game/Blueprints/Player/Animations/AM_ClimbDownEnd.AM_ClimbDownEnd"))
    (:Top
      (return (Variables|Ladder|GetTopExitLocation) (Variables|Ladder|GetTopStartLocation) (LocalVariables|GetRotation) "/Game/Blueprints/Player/Animations/AM_ClimbUpEnd.AM_ClimbUpEnd"))))