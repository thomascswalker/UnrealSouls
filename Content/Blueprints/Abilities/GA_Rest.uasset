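; GA_Rest is a Gameplay Ability that makes a Souls-style character sit and rest at a bonfire.
; On activation it disables character movement and plays the sit montage, committing the ability only once that montage completes.
; It then waits for a Character.State.Moving gameplay event on the owner to end itself.
; Ending the ability restores walking movement.
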(event Ability|EventActivateAbility
  (bind _returnvalue (Ability|GetActorInfo))
  (bind (_owneractor _avataractor _playercontroller _abilitysystemcomponent _skeletalmeshcomponent) (Utilities|Struct|BreakGameplayAbilityActorInfo _returnvalue))
  (bind _asunreal_souls_character (Utilities|Casting|CastToUnrealSoulsCharacter _owneractor))
  (Pawn|Components|CharacterMovement|SetMovementMode (Variables|/Script/Engine.Character|GetCharacterMovement _asunreal_souls_character) "MOVE_None" 0)
  (Animation|Montage|PlayMontage _skeletalmeshcomponent "/Game/Animations/Common/Resting/AM_SitAtBonfire.AM_SitAtBonfire"
    (:OnCompleted
      (Ability|CommitAbility)
      (Ability|Tasks|WaitGameplayEvent "(TagName=\"Character.State.Moving\")" _owneractor true
        (:EventReceived
          (Ability|EndAbility))))))

(event Ability|EventOnEndAbility
  (params (bWasCancelled :type Boolean))
  (bind _asunreal_souls_character (Utilities|Casting|CastToUnrealSoulsCharacter (.OwnerActor (Utilities|Struct|BreakGameplayAbilityActorInfo (Ability|GetActorInfo)))))
  (Pawn|Components|CharacterMovement|SetMovementMode (Variables|/Script/Engine.Character|GetCharacterMovement _asunreal_souls_character) "MOVE_Walking" 0))