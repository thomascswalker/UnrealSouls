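; Ladder climbing component for UnrealSoulsCharacter that handles entering, climbing and leaving a BP_Ladder.
; Start and end events pick top or bottom by distance to the bottom collider, reposition the capsule, play transition montages and switch between Flying and Walking.
; Movement input steps an alternating left/right state, playing a montage, then shifting the capsule one rung on completion.
; Tick locks yaw to the ladder; exit-collider binding is unwired.
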(event Custom|OnMovementChanged
  (params (NewMovement :type ELadderMovement%20Enum :default "None") (NewLocation :type Vector) (Montage :type Anim%20Montage%20Object%20Reference))
  (bind _characterref (Variables|Default|GetCharacterRef))
  ;[0 0 0] When the Movement value changes, play the next movement animation montage and move the character to the target location
  (Animation|Montage|PlayMontage (Variables|/Script/Engine.Character|GetMesh (Variables|Default|GetCharacterRef)) Montage (Variables|Default|GetClimbSpeed) ; Up right
    (:then
      (Variables|Default|SetbMontagePlaying true))
    (:OnCompleted
      (Variables|Default|SetbMontagePlaying false)
      (Components|MoveComponentTo (Variables|/Script/Engine.Character|GetCapsuleComponent _characterref) NewLocation (Transformation|GetActorRotation _characterref) false false 0.0 false)
      (Variables|States|SetMovement NewMovement))
    (:OnInterrupted
      (Development|PrintString "Interrupted"))))

(event Custom|OnExitTriggerOverlapped
  (params (OverlappedComponent :type Primitive%20Component%20Object%20Reference) (OtherActor :type Actor%20Object%20Reference) (OtherComp :type Primitive%20Component%20Object%20Reference) (OtherBodyIndex :type Integer) (bFromSweep :type Boolean) (SweepResult :type Hit%20Result%20Structure%20%28by%20ref%29))
  (bind _ladder (CallFunction|GetLadderBP))
  ;[0 0 0] Unbind first so we don't accidentally re-trigger the End Climb sequence
  (Utilities|IsValid _ladder
    (:Is%20Valid
      (Collision|UnbindEventfromOnComponentBeginOverlap (Variables|/Game/Blueprints/Ladders/BP_Ladder.BP_Ladder_C|GetBottomExitCollider _ladder) (EventDispatchers|CreateEvent :!event Custom|OnExitTriggerOverlapped))
      (Collision|UnbindEventfromOnComponentBeginOverlap (Variables|/Game/Blueprints/Ladders/BP_Ladder.BP_Ladder_C|GetTopExitCollider _ladder) (EventDispatchers|CreateEvent :!event Custom|OnExitTriggerOverlapped))
      (Class|ClimbingComponent|OnEndClimb))))

(event EventBeginPlay
  ;[0 0 0] Begin play
  (bind _asunreal_souls_character (Utilities|Casting|CastToUnrealSoulsCharacter (Components|GetOwner)))
  (Variables|Default|SetCharacterRef _asunreal_souls_character)
  (Class|VisualLoggerKismetLibrary|EnableRecording true))

(event EventAddMovementInput
  (params (InputValue :type Float%20%28single-precision%29))
  (bind _characterref (Variables|Default|GetCharacterRef))
  (bind _rung_height (Variables|Default|GetRung%20Height))
  (bind _characterref_2 (Variables|Default|GetCharacterRef))
  (bind _rung_height_2 (Variables|Default|GetRung%20Height))
  (bind _returnvalue (Transformation|GetActorLocation _characterref))
  (bind _returnvalue_2 (Transformation|GetActorLocation _characterref_2))
  (bind _returnvalue_3 (+ _returnvalue_2 (Math|Vector|MakeVector 0.0 0.0 _rung_height_2)))
  (bind _returnvalue_4 (- _returnvalue (Math|Vector|MakeVector 0.0 0.0 _rung_height)))
  ;[0 0 0] When the player controller provides input
  (if (not (Variables|Default|GetbMontagePlaying))
    (bind _output_get (Variables|Default|SetMovementInput InputValue))
    (if (> _output_get 0.0)
      (switch Utilities|FlowControl|Switch|SwitchonELadderMovement (Variables|States|GetMovement)
        (:Idle
          (CallFunction|OnMovementChanged "UpRight" _returnvalue_3 (Variables|Animations|GetClimbUpL) :!label _label) ; Up Left
        )
        (:UpLeft
          (goto _label))
        (:UpRight
          (CallFunction|OnMovementChanged "UpLeft" _returnvalue_3 (Variables|Animations|GetClimbUpR)) ; Up Right
        )
        (:DownLeft
          (goto _label))
        (:DownRight
          (goto _label)))
      (elif (< _output_get 0.0)
        (switch Utilities|FlowControl|Switch|SwitchonELadderMovement (Variables|States|GetMovement)
          (:Idle
            (CallFunction|OnMovementChanged "DownRight" _returnvalue_4 (Variables|Animations|GetClimbDownL) :!label _label_2) ; Down Left
          )
          (:UpLeft
            (goto _label_2))
          (:UpRight
            (goto _label_2))
          (:DownLeft
            (goto _label_2))
          (:DownRight
            (CallFunction|OnMovementChanged "DownLeft" _returnvalue_4 (Variables|Animations|GetClimbDownR)) ; Down Right
          ))))))

(event EventOnStartClimb
  (params (InLadderRef :type Ladder%20Object%20Reference))
  (bind _characterref (Variables|Default|GetCharacterRef))
  (bind _charactermovement (Variables|/Script/Engine.Character|GetCharacterMovement _characterref))
  (bind _output_get (Variables|Default|SetLadderRef InLadderRef))
  (bind _asbp_ladder (Utilities|Casting|CastToBP_Ladder _output_get))
  (Variables|Default|SetRung%20Height (Variables|/Game/Blueprints/Ladders/BP_Ladder.BP_Ladder_C|GetRungHeight _asbp_ladder))
  (Pawn|Components|CharacterMovement|SetMovementMode _charactermovement "MOVE_Flying" 0)
  (Variables|/Script/Engine.MovementComponent|SetVelocity _charactermovement "0, 0, 0")
  ;[0 0 0] Are we on the top or bottom of the ladder?
  (bind _returnvalue (CallFunction|GetOverlappingBottom))
  (if _returnvalue ; If true, overlapping bottom; else top
    (Variables|States|SetEnterTransition "ClimbUp")
    (else
      (Variables|States|SetEnterTransition "ClimbDown")))
  ;[0 0 0] Move character to starting position when entering
  (bind _transform (CallFunction|GetLadderEnterTransform))
  (Components|MoveComponentTo (Variables|/Script/Engine.Character|GetCapsuleComponent (Variables|Default|GetCharacterRef)) (.location _transform) (.rotation _transform) false false 0.2 false)
  ;[0 0 0] Play the enter transition montage
  (Animation|Montage|PlayMontage (Variables|/Script/Engine.Character|GetMesh (Variables|Default|GetCharacterRef)) (Utilities|Select :Index (Variables|States|GetEnterTransition) :ClimbUp (Variables|Animations|GetClimbUpStart) :ClimbDown (Variables|Animations|GetClimbDownStart)) (Variables|Default|GetClimbSpeed)
    (:then
      ;[0 0 0] Comment
      (Variables|Default|SetbMontagePlaying true))
    (:OnBlendOut
      (Variables|Default|SetbMontagePlaying false)
      (Variables|/Script/UnrealSouls.UnrealSoulsCharacter|SetbIsClimbing (Variables|Default|GetCharacterRef) true)
      (Variables|States|SetMovement "Idle"))))

(event EventTick
  (params (DeltaSeconds :type Float%20%28single-precision%29))
  (bind _characterref (Variables|Default|GetCharacterRef)
    (:then
      ;[0 0 0] Always rotate towards the ladder
      (bind _ladderref (Variables|Default|GetLadderRef)
        (:then
          (Transformation|SetWorldRotation (Variables|/Script/Engine.Character|GetCapsuleComponent _characterref) (Math|Rotator|MakeRotator 0.0 0.0 (.yaw (Transformation|GetActorRotation _ladderref))) false false))
        (:else)))
    (:else)))

(event EventOnEndClimb
  (bind _characterref (Variables|Default|GetCharacterRef))
  (bind _charactermovement (Variables|/Script/Engine.Character|GetCharacterMovement _characterref))
  (Variables|/Script/UnrealSouls.UnrealSoulsCharacter|SetbIsClimbing (Variables|Default|GetCharacterRef) false)
  (Variables|States|SetMovement "None")
  (bind _returnvalue (CallFunction|GetOverlappingBottom))
  (if _returnvalue ; If true, overlapping bottom; else top
    (Variables|States|SetExitTransition "ClimbDown")
    (else
      (Variables|States|SetExitTransition "ClimbUp")))
  (bind _transform (CallFunction|GetLadderExitTransform))
  (Components|MoveComponentTo (Variables|/Script/Engine.Character|GetCapsuleComponent (Variables|Default|GetCharacterRef)) (.location _transform) (.rotation _transform) false false 0.0 false)
  (Animation|Montage|PlayMontage (Variables|/Script/Engine.Character|GetMesh (Variables|Default|GetCharacterRef)) (Utilities|Select :Index (Variables|States|GetExitTransition) :ClimbUp (Variables|Animations|GetClimbUpEnd) :ClimbDown (Variables|Animations|GetClimbDownEnd)) (Variables|Default|GetClimbSpeed)
    (:then
      (Variables|Default|SetbMontagePlaying true))
    (:OnBlendOut
      (Variables|Default|SetbMontagePlaying false)
      (Pawn|Components|CharacterMovement|SetMovementMode _charactermovement "MOVE_Walking" 0)
      (Variables|/Script/Engine.CharacterMovementComponent|SetbOrientRotationToMovement _charactermovement true)
      (Variables|Default|SetLadderRef 0))))

(fn GetCharacterMovement
  (bind _characterref (Variables|Default|GetCharacterRef)
    (:then
      (return (Variables|/Script/Engine.Character|GetCharacterMovement _characterref)))
    (:else)))

(fn GetLadderEnterTransform
  (bind _ladder (CallFunction|GetLadderBP))
  (bind _entertransition (Variables|States|GetEnterTransition))
  (bind _characterref (Variables|Default|GetCharacterRef))
  (bind _capsulecomponent (Variables|/Script/Engine.Character|GetCapsuleComponent _characterref))
  (bind _topstartcomponent (Variables|/Game/Blueprints/Ladders/BP_Ladder.BP_Ladder_C|GetTopStartComponent _ladder))
  (bind _bottomstartcomponent (Variables|/Game/Blueprints/Ladders/BP_Ladder.BP_Ladder_C|GetBottomStartComponent _ladder))
  (bind _returnvalue (Transformation|GetWorldLocation _capsulecomponent))
  (bind _returnvalue_2 (Utilities|Select :Index _entertransition :ClimbUp _bottomstartcomponent :ClimbDown _topstartcomponent))
  (bind _returnvalue_3 (Transformation|GetWorldLocation _returnvalue_2))
  (bind _returnvalue_4 (Math|Vector|MakeVector (.x _returnvalue_3) (.y _returnvalue_3) (.z _returnvalue)))
  (Class|VisualLoggerKismetLibrary|LogLocation 0 _returnvalue_4 "EnterLocation" "(R=1.000000,G=0.000000,B=0.000000,A=1.000000)" 1e+01 "ClimbingComponent")
  (return (Math|Transform|MakeTransform _returnvalue_4 (Math|Rotator|MakeRotator 0.0 0.0 (.yaw (Transformation|GetActorRotation (Variables|Default|GetLadderRef)))) "1.000000,1.000000,1.000000")))

(fn GetLadderExitTransform
  (bind _ladder (CallFunction|GetLadderBP))
  (bind _characterref (Variables|Default|GetCharacterRef))
  (bind _exittransition (Variables|States|GetExitTransition))
  (bind _bottomexitcomponent (Variables|/Game/Blueprints/Ladders/BP_Ladder.BP_Ladder_C|GetBottomExitComponent _ladder))
  (bind _topstartcomponent (Variables|/Game/Blueprints/Ladders/BP_Ladder.BP_Ladder_C|GetTopStartComponent _ladder))
  (bind _capsulecomponent (Variables|/Script/Engine.Character|GetCapsuleComponent _characterref))
  (bind _returnvalue (Components|Capsule|GetScaledCapsuleHalfHeight _capsulecomponent))
  (bind _returnvalue_2 (Utilities|Select :Index _exittransition :ClimbUp _topstartcomponent :ClimbDown _bottomexitcomponent))
  (bind _returnvalue_3 (Transformation|GetWorldLocation _returnvalue_2))
  (bind _returnvalue_4 (+ _returnvalue_3 (Math|Vector|MakeVector 0.0 0.0 _returnvalue)))
  (Class|VisualLoggerKismetLibrary|LogLocation 0 _returnvalue_4 "ExitLocation" "(R=1.000000,G=0.000000,B=0.000000,A=1.000000)" 1e+01 "ClimbingComponent")
  (return (Math|Transform|MakeTransform _returnvalue_4 (Math|Rotator|MakeRotator 0.0 0.0 (.yaw (Transformation|GetActorRotation (Variables|Default|GetLadderRef)))) "1.000000,1.000000,1.000000")))

(fn GetLadderBP
  (bind _ladderref (Variables|Default|GetLadderRef)
    (:then
      (bind _asbp_ladder (Utilities|Casting|CastToBP_Ladder _ladderref))
      (return _asbp_ladder))
    (:else)))

(fn GetOverlappingBottom
  (return (< (Math|Vector|VectorLength (- (Transformation|GetWorldLocation (Variables|/Script/Engine.Character|GetCapsuleComponent (Variables|Default|GetCharacterRef))) (Transformation|GetWorldLocation (Variables|/Game/Blueprints/Ladders/BP_Ladder.BP_Ladder_C|GetBottomExitCollider (CallFunction|GetLadderBP))))) 2e+02)))

(fn GetLadderData
  (bind _bmontageplaying (Variables|Default|GetbMontagePlaying))
  (return (Utilities|Struct|MakeLadderData (Variables|States|GetEnterTransition) (Variables|States|GetExitTransition) (Variables|States|GetMovement) _bmontageplaying _bmontageplaying (Variables|Default|GetMovementInput) (CallFunction|GetLadderBP) (Variables|Default|GetCharacterRef))))