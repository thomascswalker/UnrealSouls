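; AN_LadderMove is an anim notify that updates the climbing character's ladder movement state.
; It resolves the mesh owner's Instigator to an UnrealSoulsCharacter and its BP_ClimbingComponent, caching that component, the ladder and its data.
; With non-zero vertical velocity, it alternates Movement between UpLeft and UpRight based on the ladder data, leaving Idle unchanged.
; With zero vertical velocity, it sets Movement to Idle.
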(fn ReceivedNotify
  (params (MeshComp :type Skeletal%20Mesh%20Component%20Object%20Reference) (Animation :type Anim%20Sequence%20Base%20Object%20Reference) (EventReference :type Anim%20Notify%20Event%20Reference%20Structure%20%28by%20ref%29))
  (bind _instigator (Variables|/Script/Engine.Actor|GetInstigator (Components|GetOwner MeshComp))
    (:then
      (bind _asunreal_souls_character (Utilities|Casting|CastToUnrealSoulsCharacter _instigator))
      (bind _asbp_climbing_component (Utilities|Casting|CastToBP_ClimbingComponent (Variables|/Script/UnrealSouls.UnrealSoulsCharacter|GetClimbingComponent _asunreal_souls_character)))
      (bind _output_get (LocalVariables|SetClimbingComponentRef _asbp_climbing_component))
      (LocalVariables|SetLadderRef (Default|GetLadderBP _output_get))
      (bind _data (Default|GetLadderData _output_get))
      (LocalVariables|SetLadderDataRef _data)
      (if (!= (.z (Transformation|GetVelocity (Components|GetOwner (LocalVariables|GetClimbingComponentRef)))) 0.0)
        (switch Utilities|FlowControl|Switch|SwitchonELadderMovement (.Movement (Utilities|Struct|BreakLadderData (LocalVariables|GetLadderDataRef)))
          (:Idle
            (return false))
          (:UpLeft
            (Variables|/Game/Blueprints/Components/BP_ClimbingComponent.BP_ClimbingComponent_C|SetMovement (LocalVariables|GetClimbingComponentRef) "UpRight"))
          (:UpRight
            (Variables|/Game/Blueprints/Components/BP_ClimbingComponent.BP_ClimbingComponent_C|SetMovement (LocalVariables|GetClimbingComponentRef) "UpLeft")))
        (return true)
        (else
          (Variables|/Game/Blueprints/Components/BP_ClimbingComponent.BP_ClimbingComponent_C|SetMovement (LocalVariables|GetClimbingComponentRef) "Idle")
          (return false))))
    (:else)))