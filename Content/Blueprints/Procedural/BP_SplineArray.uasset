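; Procedural chain actor that builds a run of links along a spline in the construction script.
; It adds instanced link meshes at even distances between start and end offsets, with LinkCount setting the density.
; Every other link is rotated 90 degrees so the chain appears interlocked.
; Optional start and end cap meshes sit on the first and last spline points with an adjustable rotation offset.
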(event EventBeginPlay)

(event Collision|EventActorBeginOverlap
  (params (OtherActor :type Actor%20Object%20Reference)))

(event EventTick
  (params (DeltaSeconds :type Float%20%28single-precision%29)))

(fn ConstructionScript
  (Utilities|FlowControl|Sequence
    (:then_0
      ;[0 0 0] Start
      (if (Variables|ChainOptions|GetbUseStart)
        (bind _returnvalue (AddComponent|AddStaticMeshComponent false (CallFunction|GetPointTransform)))
        (Components|StaticMesh|SetStaticMesh _returnvalue "/Game/Blueprints/Procedural/SM_Chain_Start.SM_Chain_Start")))
    (:then_1
      ;[0 0 0] Middle
      (bind _returnvalue_2 (AddComponent|AddInstancedStaticMeshComponent false))
      (Components|StaticMesh|SetStaticMesh _returnvalue_2 "/Game/Blueprints/Procedural/SM_Chain_Link.SM_Chain_Link")
      (for _index (range 0 (Variables|ChainOptions|GetLinkCount))
        (Components|InstancedStaticMesh|AddInstance _returnvalue_2 (CallFunction|GetLinkTransform _index) false)))
    (:then_2
      ;[0 0 0] End
      (if (Variables|ChainOptions|GetbUseEnd)
        (bind _returnvalue_3 (AddComponent|AddStaticMeshComponent false (CallFunction|GetPointTransform (- (Spline|GetNumberOfSplinePoints (Variables|Default|GetSpline)) 1))))
        (Components|StaticMesh|SetStaticMesh _returnvalue_3 "/Game/Blueprints/Procedural/SM_Chain_End.SM_Chain_End")))))

(fn GetPointTransform
  (params (PointIndex :type Integer))
  (bind _spline (Variables|Default|GetSpline))
  (bind _returnvalue (Spline|GetTransformatSplinePoint _spline PointIndex "Local" false))
  (return (Math|Transform|MakeTransform (.location _returnvalue) (Math|Rotator|CombineRotators (.rotation _returnvalue) (Variables|ChainOptions|Offset|GetOffsetRotation)) (.scale _returnvalue))))

(fn GetLinkTransform
  (params (Index :type Integer))
  (bind _returnvalue (Math|Conversions|ToFloat(Integer) Index))
  (bind _spline (Variables|Default|GetSpline))
  (bind _spline_2 (Variables|Default|GetSpline))
  (bind _linkcount (Variables|ChainOptions|GetLinkCount))
  (bind _startoffset (Variables|ChainOptions|Offset|GetStartOffset))
  (bind _endoffset (Variables|ChainOptions|Offset|GetEndOffset))
  (bind _returnvalue_2 (Spline|GetSplineLength _spline))
  (bind _returnvalue_3 (Math|Conversions|ToFloat(Integer) _linkcount))
  (bind _returnvalue_4 (/ _returnvalue _returnvalue_3))
  (bind _returnvalue_5 (- _returnvalue_2 _endoffset))
  (bind _returnvalue_6 (* _returnvalue_4 _returnvalue_2))
  (bind _returnvalue_7 (Math|Float|MapRangeClamped _returnvalue_6 0.0 _returnvalue_2 _startoffset _returnvalue_5))
  (bind _returnvalue_8 (Spline|GetTransformatDistanceAlongSpline _spline_2 _returnvalue_7 "Local" false))
  (return (Math|Transform|MakeTransform (.location _returnvalue_8) (Math|Rotator|CombineRotators (Math|Rotator|SelectRotator "0.000000,0.000000,90.000000" "0, 0, 0" (== (Math|Integer|%(Integer) Index 2) 0)) (.rotation _returnvalue_8)) "1.000000,1.000000,1.000000")))