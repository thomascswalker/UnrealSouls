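; BP_EntitySpawn is an enemy spawn marker that shows a Hollow skeletal mesh as a placement preview.
; The construction script adds the mesh, lowers it by its bounds half-height and copies the actor's rotation into its relative rotation.
; BeginPlay calls the parent, then destroys the preview component; no spawning logic lives in this Blueprint.
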(event EventBeginPlay
  (|CallParentFunction)
  (Components|DestroyComponent (Variables|Default|GetNewVar)))

(fn ConstructionScript
  (|CallParentFunction)
  (bind _returnvalue (AddComponent|AddSkeletalMeshComponent false))
  (bind _output_get (Variables|Default|SetNewVar _returnvalue))
  (Components|SkeletalMesh|SetSkeletalMeshAsset _output_get "/Game/Characters/Hollow/SK_Hollow.SK_Hollow")
  (Transformation|AddLocalOffset _output_get (Math|Vector|MakeVector 0.0 0.0 (* (.z (.boxextent (StaticMesh|GetBounds (Variables|/Script/Engine.SkeletalMeshComponent|GetSkeletalMeshAsset _output_get)))) -1.0)) false false)
  (Transformation|SetRelativeRotation _output_get (Transformation|GetActorRotation) false false))