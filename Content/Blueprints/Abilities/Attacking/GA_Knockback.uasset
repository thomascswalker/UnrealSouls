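; GA_Knockback is a gameplay ability that knocks a living souls-like character backward with a hit reaction.
; On activation it casts the owner to UnrealSoulsCharacter, checks it is alive, and plays the AM_Hit montage on its mesh.
; As the montage starts, it launches the character along its negated horizontal forward vector scaled by KnockbackIntensity, overriding velocity, and ends the ability when the montage completes.
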(event Ability|EventActivateAbility
  (bind _asunreal_souls_character (Utilities|Casting|CastToUnrealSoulsCharacter (.OwnerActor (Utilities|Struct|BreakGameplayAbilityActorInfo (Ability|GetActorInfo)))))
  (if (Class|UnrealSoulsCharacter|IsAlive _asunreal_souls_character)
    (Animation|Montage|PlayMontage (Variables|/Script/Engine.Character|GetMesh _asunreal_souls_character) "/Game/Animations/Common/Combat/AM_Hit.AM_Hit"
      (:then
        (Character|LaunchCharacter _asunreal_souls_character (* (Math|Vector|MakeVector (* (.x (Transformation|GetActorForwardVector _asunreal_souls_character)) -1.0) (* (.y (Transformation|GetActorForwardVector _asunreal_souls_character)) -1.0) 0.0) (Variables|Default|GetKnockbackIntensity)) true true))
      (:OnCompleted
        (Ability|EndAbility)))))

(event Ability|EventOnEndAbility
  (params (bWasCancelled :type Boolean)))