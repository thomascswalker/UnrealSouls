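; Player character Blueprint for a Souls-like game, handling HUD, bonfire resting, death and modular armor meshes.
; BeginPlay creates the HUD, binds resting and death events, and moves the audio listener to the capsule.
; Resting toggles the bonfire menu and input mode, while sitting animates a post-process material blend on the follow camera.
; Death plays an invulnerable montage before destroying the actor, and overrides supply hitbox, character type and health bar.
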(event Custom|RestingStateChanged
  (params (bRestingState :type Boolean))
  ;[0 0 0] Bonfire menu
  (if bRestingState
    (bind _returnvalue (UserInterface|CreateWidget "/Game/Blueprints/HUD/WBP_BonfireMenu.WBP_BonfireMenu_C"))
    (bind _output_get (Variables|Default|SetBonfireMenu _returnvalue))
    (UserInterface|Viewport|AddtoViewport _output_get 0)
    (bind _returnvalue_2 (Class|PlayerFunctionLibrary|GetPlayerController))
    (Variables|/Script/Engine.PlayerController|SetbShowMouseCursor _returnvalue_2 true)
    (Input|SetInputModeUIOnly _returnvalue_2 _output_get "DoNotLock" false)
    (else
      (bind _bonfiremenu (Variables|Default|GetBonfireMenu)
        (:then
          (Widget|RemovefromParent _bonfiremenu)
          (bind _returnvalue_3 (Class|PlayerFunctionLibrary|GetPlayerController))
          (Variables|/Script/Engine.PlayerController|SetbShowMouseCursor _returnvalue_3 false)
          (Input|SetInputModeGameOnly _returnvalue_3 false))
        (:else)))))

(event Custom|OnBonfireSitStarted
  (bind _bonfirescreenmaterial (Variables|Default|GetBonfireScreenMaterial))
  ;[0 0 0] Bonfire screen animation
  (bind _bonfirescreenvisibility (Timeline|Timeline PlayFromStart)
    (:Update
      (Rendering|Material|SetScalarParameterValue _bonfirescreenmaterial "Blend" _bonfirescreenvisibility :!class /Script/Engine.MaterialInstanceDynamic)
      (Variables|/Script/Engine.CameraComponent|SetPostProcessSettings (Variables|Default|GetFollowCamera) (Utilities|Struct|MakePostProcessSettings (Utilities|Struct|MakeWeightedBlendables (Utilities|Array|MakeArray (Utilities|Struct|MakeWeightedBlendable 1.0 _bonfirescreenmaterial))))))))

(event Custom|OnDeath
  ;[1 0 0] Death
  (Animation|Montage|PlayMontage (Variables|Character|GetMesh) "/Game/Animations/Common/Combat/ARPG_Warrior_Anim_UE_Death3_Montage.ARPG_Warrior_Anim_UE_Death3_Montage"
    (:then
      (Class|CombatInterface|SetInvulnerable true))
    (:OnCompleted
      (Actor|DestroyActor :!label _label))
    (:OnBlendOut
      (goto _label))))

(event EventBeginPlay
  (|CallParentFunction)
  (Utilities|FlowControl|Sequence
    (:then_0
      ;[0 0 0] Main HUD widget
      (bind _returnvalue (UserInterface|CreateWidget "/Game/Blueprints/HUD/WBP_MainHUD.WBP_MainHUD_C" 0 self))
      (bind _output_get (Variables|Default|SetMainHud _returnvalue))
      (UserInterface|Viewport|AddtoViewport _output_get 0))
    (:then_1
      ;[0 0 0] Binding events
      (EventDispatchers|BindEventtoRestingChanged (EventDispatchers|CreateEvent :!event Custom|RestingStateChanged))
      (EventDispatchers|BindEventtoDied (EventDispatchers|CreateEvent :!event Custom|OnDeath)))
    (:then_2
      ;[0 0 0] Audio Override
      (bind _returnvalue_2 (Class|PlayerFunctionLibrary|GetPlayerController))
      (Class|PlayerController|SetAudioListenerOverride _returnvalue_2 (Variables|Default|GetCapsuleComponent) "0, 0, 0" "0, 0, 0"))
    (:then_3
      ;[0 0 0] Bonfire screen material
      (bind _returnvalue_3 (Rendering|Material|CreateDynamicMaterialInstance "/Game/Materials/Interface/M_BonfireScreen.M_BonfireScreen" "None" "None" :!class /Script/Engine.KismetMaterialLibrary))
      (Variables|Default|SetBonfireScreenMaterial _returnvalue_3)
      (Development|PrintString (Utilities|String|ToString(Float) (.ReturnValue (Class|AbilitySystemComponent|GetGameplayAttributeValue (Variables|Default|GetAbilitySystemComponent) "(AttributeName=\"AttackPower\",Attribute=/Script/UnrealSouls.CharacterAttributeSet:AttackPower,AttributeOwner=/Script/CoreUObject.Class'\"/Script/UnrealSouls.CharacterAttributeSet\"')")))))))

(fn ConstructionScript
  (|CallParentFunction)
  (Components|SkinnedMesh|SetLeaderPoseComponent (Variables|Default|GetArmorMesh) (Variables|Character|GetMesh) false false)
  (Components|SkinnedMesh|SetLeaderPoseComponent (Variables|Default|GetLegsMesh) (Variables|Character|GetMesh) false false)
  (Components|SkinnedMesh|SetLeaderPoseComponent (Variables|Default|GetHandsMesh) (Variables|Character|GetMesh) false false)
  (Transformation|AttachComponentToComponent (Variables|Default|GetHelmetMesh) (Variables|Character|GetMesh) "head" "KeepRelative" "KeepRelative" "KeepRelative" true))

(fn GetWeaponHitbox
  (return (Variables|Default|GetCapsule)))

(fn GetCharacterTypeMask
  (return "Player"))

(fn GetHealthBarWidget
  (return (Variables|/Game/Blueprints/HUD/WBP_MainHUD.WBP_MainHUD_C|GetHealthBar (Variables|Default|GetMainHud))))