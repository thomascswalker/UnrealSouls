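; AN_AttackStart is an animation notify that performs a melee hit check when an attack animation reaches it.
; When the mesh owner is an UnrealSoulsCharacter, it runs a single zero-length sphere trace at the right-hand socket on the Visibility channel.
; A hit UnrealSoulsCharacter receives fixed damage through OnTakeDamage.
; Debug drawing and a placeholder print message are left in.
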(fn ReceivedNotify
  (params (MeshComp :type Skeletal%20Mesh%20Component%20Object%20Reference) (Animation :type Anim%20Sequence%20Base%20Object%20Reference) (EventReference :type Anim%20Notify%20Event%20Reference%20Structure%20%28by%20ref%29))
  (bind _returnvalue (Transformation|GetSocketLocation MeshComp "hand_rSocket"))
  (Utilities|Casting|CastToUnrealSoulsCharacter (Components|GetOwner MeshComp))
  (bind _outhit (Collision|SphereTraceByChannel _returnvalue _returnvalue 25.0 "TraceTypeQuery1" false 0 "ForDuration" true "(R=1.000000,G=0.000000,B=0.000000,A=1.000000)" "(R=0.000000,G=1.000000,B=0.000000,A=1.000000)" 2.0))
  (bind _asunreal_souls_character (Utilities|Casting|CastToUnrealSoulsCharacter (.HitActor (Collision|BreakHitResult _outhit)))
    (:then
      (Class|UnrealSoulsCharacter|OnTakeDamage _asunreal_souls_character 5.0)
      (Development|PrintString "Hello")
      (return true))
    (:CastFailed
      (return false))))