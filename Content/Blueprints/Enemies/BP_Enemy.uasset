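; BP_Enemy is an enemy that chases the player on sight and starts an attack.
; Its PawnSensing component stores a seen UnrealSoulsPlayerCharacter as the target, sets a seeing flag and calls FollowPlayer.
; FollowPlayer runs AI MoveTo toward player pawn 0 and calls the CombatComponent's attack start from the node's immediate Then output, without waiting for arrival.
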(event OnSeePawn(PawnSensing)
  (params (Pawn :type Pawn%20Object%20Reference))
  (bind _asunreal_souls_player_character (Utilities|Casting|CastToUnrealSoulsPlayerCharacter Pawn))
  (Variables|Default|SetTarget _asunreal_souls_player_character)
  (Variables|Default|SetbIsSeeingPlayer true)
  (CallFunction|FollowPlayer))

(event Custom|FollowPlayer
  (if (Variables|Default|GetbIsSeeingPlayer)
    (AI|AIMoveTo self "0, 0, 0" (Game|Player|GetPlayerPawn 0) 15.0 false
      (:then
        (Class|CombatComponent|OnAttackStart (Variables|Default|GetCombatComponent))))))

(fn ConstructionScript)