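; Base enemy character Blueprint that feeds player perception to its AI and handles its own death.
; PawnSensing writes whether the seen player is resting, is visible and is within attack distance to the AI controller's Blackboard.
; BeginPlay binds to the Died event, and OnDeath plays a death montage, destroying the actor when it completes or blends out.
; Getter functions supply the capsule weapon hitbox and the Enemy character type.
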(event OnSeePawn(PawnSensing)
  (params (Pawn :type Pawn%20Object%20Reference))
  (bind _self self)
  (bind _returnvalue (AI|GetAIController _self))
  (bind _returnvalue_2 (AI|GetBlackboard _returnvalue))
  (bind _asunreal_souls_player_character (Utilities|Casting|CastToUnrealSoulsPlayerCharacter Pawn))
  ;[0 0 0] bPlayerResting
  (AI|Components|Blackboard|SetValueasBool (AI|GetBlackboard (AI|GetAIController self)) (Utilities|Name|MakeLiteralName "bPlayerResting") (Class|UnrealSoulsCharacter|IsResting _asunreal_souls_player_character))
  ;[0 0 0] bSeesPlayer
  (AI|Components|Blackboard|SetValueasBool _returnvalue_2 (Utilities|Name|MakeLiteralName "bSeesPlayer") true)
  (AI|Components|Blackboard|SetValueasBool _returnvalue_2 (Utilities|Name|MakeLiteralName "bCanAttack") (< (Math|Vector|Distance(Vector) (Transformation|GetActorLocation _asunreal_souls_player_character) (Transformation|GetActorLocation)) (Variables|Default|GetAttackDistanceThreshold))))

(event Custom|OnDeath
  (Animation|Montage|PlayMontage (Variables|Character|GetMesh) "/Game/Animations/Common/Combat/ARPG_Warrior_Anim_UE_Death3_Montage.ARPG_Warrior_Anim_UE_Death3_Montage"
    (:OnCompleted
      _)
    (:OnBlendOut
      _))
  (Actor|DestroyActor))

(event EventBeginPlay
  (|CallParentFunction)
  (EventDispatchers|BindEventtoDied (EventDispatchers|CreateEvent :!event Custom|OnDeath)))

(fn ConstructionScript)

(fn GetWeaponHitbox
  (return (Variables|Default|GetCapsule)))

(fn GetCharacterTypeMask
  (return "Enemy"))