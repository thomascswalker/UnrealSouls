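; MyStaticEntity is an interactable entity that shows an action prompt, "Climb", when the Souls-style player character is near.
; Its capsule's overlap events cast to the player character and its controller, showing the prompt on entry and hiding it on exit.
; GetActionText supplies the prompt label, and the Blueprint contains no climbing logic itself.
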(event OnComponentBeginOverlap(CapsuleComponent)
  (params (OverlappedComponent :type Primitive%20Component%20Object%20Reference) (OtherActor :type Actor%20Object%20Reference) (OtherComp :type Primitive%20Component%20Object%20Reference) (OtherBodyIndex :type Integer) (bFromSweep :type Boolean) (SweepResult :type Hit%20Result%20Structure%20%28by%20ref%29))
  (bind _asbp_unreal_souls_player_character (Utilities|Casting|CastToBP_UnrealSoulsPlayerCharacter OtherActor))
  (bind _asbp_unreal_souls_player_controller (Utilities|Casting|CastToBP_UnrealSoulsPlayerController (Pawn|GetController _asbp_unreal_souls_player_character)))
  (Default|ShowPrompt _asbp_unreal_souls_player_controller (CallFunction|GetActionText)))

(event OnComponentEndOverlap(CapsuleComponent)
  (params (OverlappedComponent :type Primitive%20Component%20Object%20Reference) (OtherActor :type Actor%20Object%20Reference) (OtherComp :type Primitive%20Component%20Object%20Reference) (OtherBodyIndex :type Integer))
  (bind _asbp_unreal_souls_player_character (Utilities|Casting|CastToBP_UnrealSoulsPlayerCharacter OtherActor))
  (bind _asbp_unreal_souls_player_controller (Utilities|Casting|CastToBP_UnrealSoulsPlayerController (Pawn|GetController _asbp_unreal_souls_player_character)))
  (Default|HidePrompt _asbp_unreal_souls_player_controller))

(fn ConstructionScript)

(fn GetActionText
  (return "Climb"))