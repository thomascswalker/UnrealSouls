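; GA_Roll is the gameplay ability that makes an UnrealSoulsCharacter perform a forward dodge roll.
; On activation it commits, applies the GE_IsRolling effect, plays the forward roll montage, and launches the character along the capsule's forward vector scaled by RollSpeed.
; The ability ends when the montage completes, blends out or is interrupted, then removes effects granting the IsRolling tag.
; A ContinueRoll event exists but is empty.
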(event Custom|ContinueRoll)

(event Ability|EventActivateAbility
  (bind _returnvalue (Ability|GetActorInfo))
  (bind (_owneractor _avataractor _playercontroller _abilitysystemcomponent _skeletalmeshcomponent) (Utilities|Struct|BreakGameplayAbilityActorInfo _returnvalue))
  (Ability|CommitAbility)
  (Ability|ApplyGameplayEffectToOwner "/Game/Blueprints/Abilities/GE_IsRolling.GE_IsRolling_C")
  (Animation|Montage|PlayMontage _skeletalmeshcomponent "/Game/Blueprints/Player/Animations/AM_RollForward.AM_RollForward"
    (:then
      (bind _asunreal_souls_character (Utilities|Casting|CastToUnrealSoulsCharacter _owneractor))
      (Character|LaunchCharacter _asunreal_souls_character (* (Math|Vector|GetForwardVector (Variables|/Script/Engine.Character|GetCapsuleComponent _asunreal_souls_character)) (Variables|Default|GetRollSpeed)) false false))
    (:OnCompleted
      (Ability|EndAbility :!label _label))
    (:OnBlendOut
      (goto _label))
    (:OnInterrupted
      (goto _label))))

(event Ability|EventOnEndAbility
  (params (bWasCancelled :type Boolean))
  (Ability|RemoveGameplayEffectFromOwnerWithGrantedTags "(GameplayTags=((TagName=\"Character.State.IsRolling\")))"))